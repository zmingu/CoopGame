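; Health regeneration powerup that heals every SCharacter in the level by HealAmount on each powerup tick.
; Activation makes its static mesh visible.
; Each tick gathers all SCharacter actors and calls Heal on any valid SHealthComponent, with no filter for who picked it up.
; Tick timing is not set in this graph, which only responds to the OnActivated and OnPowerUpTicked events.
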(event EventBeginPlay
  (|CallParentFunction) ; 此节点被禁用，将不会被调用。\n从引脚连出引线来编译功能。
)

(event Collision|EventActorBeginOverlap
  (params (OtherActor :type Actor%20Object%20Reference))
  (|CallParentFunction OtherActor) ; 此节点被禁用，将不会被调用。\n从引脚连出引线来编译功能。
)

(event EventTick
  (params (DeltaSeconds :type Float%20%28single-precision%29))
  (|CallParentFunction DeltaSeconds) ; 此节点被禁用，将不会被调用。\n从引脚连出引线来编译功能。
)

(event EventOnActivated
  (Rendering|SetVisibility (Variables|Default|GetStaticMesh) true false))

(event EventOnPowerUpTicked
  (bind _outactors (Actor|GetAllActorsOfClass "/Script/CoopGame.SCharacter"))
  (for _array_element _outactors
    (Utilities|IsValid (Actor|GetComponentbyClass _array_element "/Script/CoopGame.SHealthComponent")
      (:Is%20Valid
        (Class|SHealthComponent|Heal (Actor|GetComponentbyClass _array_element "/Script/CoopGame.SHealthComponent") (Variables|Default|GetHealAmount))))))

(fn ConstructionScript
  (|CallParentFunction))