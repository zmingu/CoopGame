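; Super speed powerup that temporarily doubles the walk speed of the player it activates for.
; On activation it stores the target player, hides its mesh and sets MaxWalkSpeed to twice the movement component's current max speed.
; On expiry it shows the mesh, sets MaxWalkSpeed to half the current max speed rather than restoring a saved value, then destroys itself.
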(event EventBeginPlay
  (|CallParentFunction) ; 此节点被禁用，将不会被调用。\n从引脚连出引线来编译功能。
)

(event Collision|EventActorBeginOverlap
  (params (OtherActor :type Actor%20Object%20Reference))
  (|CallParentFunction OtherActor) ; 此节点被禁用，将不会被调用。\n从引脚连出引线来编译功能。
)

(event EventTick
  (params (DeltaSeconds :type Float%20%28single-precision%29))
  (|CallParentFunction DeltaSeconds) ; 此节点被禁用，将不会被调用。\n从引脚连出引线来编译功能。
)

(event EventOnExpired
  (bind _active_target_player (Variables|Default|GetActive%20Target%20Player))
  (bind _returnvalue (Actor|GetComponentbyClass _active_target_player "/Script/Engine.CharacterMovementComponent"))
  (Rendering|SetVisibility (Variables|Default|GetStaticMesh) true false)
  (Variables|/Script/Engine.CharacterMovementComponent|SetMaxWalkSpeed _returnvalue (/ (Class|MovementComponent|GetMaxSpeed _returnvalue) 2.0))
  (Actor|DestroyActor))

(event EventOnActivated
  (params (ActiveFor :type Actor%20Object%20Reference))
  (bind _output_get (Variables|Default|SetActive%20Target%20Player ActiveFor))
  (Rendering|SetVisibility (Variables|Default|GetStaticMesh) false false)
  (Variables|/Script/Engine.CharacterMovementComponent|SetMaxWalkSpeed (Actor|GetComponentbyClass _output_get "/Script/Engine.CharacterMovementComponent") (* (Class|MovementComponent|GetMaxSpeed (Actor|GetComponentbyClass _output_get "/Script/Engine.CharacterMovementComponent")) 2.0)))

(fn ConstructionScript
  (|CallParentFunction))